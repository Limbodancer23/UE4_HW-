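; BP_SimpleBall is a ball actor that travels in straight lines and bounces off whatever blocks it.
; Each Tick, it makes a swept world offset along its direction Vector, scaled by Speed and delta time, without physics forces.
; A blocking hit mirrors that Vector around the hit normal, setting the direction for later frames.
; Overlapping a KillZVolume destroys the ball.
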(event EventBeginPlay)

(event Collision|EventActorBeginOverlap
  (params (OtherActor :type Actor%20Object%20Reference))
  (Utilities|Casting|CastToKillZVolume OtherActor)
  (Actor|DestroyActor))

(event EventTick
  (params (DeltaSeconds :type Float%20%28single-precision%29))
  (bind _sweephitresult (Transformation|AddActorWorldOffset (* (* (Variables|Default|GetVector) (Variables|Default|GetSpeed)) DeltaSeconds) true))
  (if (.bBlockingHit (Collision|BreakHitResult _sweephitresult))
    (Variables|Default|SetVector (Math|Vector|GetReflectionVector (Variables|Default|GetVector) (.Normal (Collision|BreakHitResult _sweephitresult))))))

(fn ConstructionScript)