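; BP_Blocks is a breakable brick field for a ball game that tracks the win condition.
; The construction script builds a grid of static mesh blocks, randomly making about 4% unbreakable and counting the rest.
; A BP_SimpleBall hit first swaps a breakable block's material, then a second destroys it, spawning a BP_Bonus and decrementing the count.
; Material comparison serves as block state, and zero remaining prints a win message.
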(event EventBeginPlay)

(event Collision|EventActorBeginOverlap
  (params (OtherActor :type Actor%20Object%20Reference)))

(event EventTick
  (params (DeltaSeconds :type Float%20%28single-precision%29)))

(event Collision|EventHit
  (params (MyComp :type Primitive%20Component%20Object%20Reference) (Other :type Actor%20Object%20Reference) (OtherComp :type Primitive%20Component%20Object%20Reference) (bSelfMoved :type Boolean) (HitLocation :type Vector :default "0, 0, 0") (HitNormal :type Vector :default "0, 0, 0") (NormalImpulse :type Vector :default "0, 0, 0") (Hit :type Hit%20Result%20Structure%20%28by%20ref%29))
  (bind _returnvalue (Rendering|Material|GetMaterial MyComp 0))
  (bind _material (Variables|Default|GetMaterial))
  (Utilities|Casting|CastToBP_SimpleBall Other)
  (if (not (== (Variables|Default|GetDestruct) _returnvalue))
    (if (== _returnvalue _material)
      (bind _output_get (Variables|Default|SetLocation (Transformation|GetWorldLocation MyComp)))
      (Components|DestroyComponent MyComp)
      (CallFunction|SpawnBonus _output_get)
      (bind _result (Math|Integer|DecrementInt (Variables|Default|GetCount))
        (:%20%20
          (bind _output_get_2 (Variables|Default|SetCount _result))
          (if (== _result 0)
            (Development|PrintString "You win!!" true true "(R=1.000000,G=0.117468,B=0.287726,A=1.000000)" 1e+01)
            (else
              (Development|PrintString (Utilities|String|ToString(Integer) _output_get_2))))))
      (else
        (Rendering|Material|SetMaterial MyComp 0 _material)))))

(fn ConstructionScript
  (for _index (range 0 (Variables|Default|GetX))
    (for _index_2 (range 0 (Variables|Default|GetY))
      (if (>= (Math|Random|RandomInteger 100) 96)
        (bind _returnvalue (AddComponent|AddStaticMeshComponent false (Math|Transform|MakeTransform (Math|Vector|MakeVector (Math|Conversions|ToFloat(Integer) (* _index (Variables|Default|GetPadding))) (Math|Conversions|ToFloat(Integer) (* _index_2 (Variables|Default|GetPadding))) 0.0))))
        (Variables|Default|SetDestruct (Rendering|Material|GetMaterial _returnvalue 0))
        (else
          (bind _result (Math|Integer|IncrementInt (Variables|Default|GetCount))
            (:%20%20
              (AddComponent|AddStaticMeshComponent false (Math|Transform|MakeTransform (Math|Vector|MakeVector (Math|Conversions|ToFloat(Integer) (* _index (Variables|Default|GetPadding))) (Math|Conversions|ToFloat(Integer) (* _index_2 (Variables|Default|GetPadding))) 0.0))))))))))

(fn SpawnBonus
  (params (Spawn%20Transform%20Location :type Vector))
  (bind _returnvalue (Game|SpawnActorfromClass "/Game/BP_Bonus.BP_Bonus_C" (Math|Transform|MakeTransform Spawn%20Transform%20Location "0, 0, 0" "1,1,1") "AlwaysSpawn" 0 0))
  (Variables|Default|SetNewBon _returnvalue)
  (return))