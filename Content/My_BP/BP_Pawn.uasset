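; Player paddle pawn for a ball game that moves sideways and spawns balls.
; MoveRight input applies fixed swept world-Y steps opposite to the axis sign, without delta-time scaling.
; BeginPlay spawns the main ball at the capsule, stores it and binds to its OnDeadBall event.
; Overlapping a BP_Bonus spawns an additional BP_SimpleBall at the capsule.
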(event EventBeginPlay
  (CallFunction|SpawnBall))

(event Collision|EventActorBeginOverlap
  (params (OtherActor :type Actor%20Object%20Reference))
  (Utilities|Casting|CastToBP_Bonus OtherActor)
  (CallFunction|SpawnAnother))

(event EventTick
  (params (DeltaSeconds :type Float%20%28single-precision%29)))

(event Input|AxisEvents|InputAxisMoveRight
  (params (AxisValue :type Float%20%28single-precision%29))
  (if (< AxisValue 0.0)
    (Transformation|AddActorWorldOffset "0,50.000000, 0" true)))

(event Input|AxisEvents|InputAxisMoveRight
  (params (AxisValue :type Float%20%28single-precision%29))
  (if (> AxisValue 0.0)
    (Transformation|AddActorWorldOffset "0,-50.000000, 0" true)))

(fn ConstructionScript)

(fn SpawnBall
  (bind _returnvalue (Game|SpawnActorfromClass "/Game/My_BP/BP_MainBall.BP_MainBall_C" (Math|Transform|MakeTransform (Transformation|GetWorldLocation (Variables|Default|GetCapsule)) "0, 0, 0" "1,1,1") "AlwaysSpawn" 0 0))
  (bind _output_get (Variables|Default|SetPlayingBall _returnvalue))
  (EventDispatchers|BindEventtoOnDeadBall _output_get (EventDispatchers|CreateEvent :!event SpawnBall))
  (return))

(fn SpawnAnother
  (bind _returnvalue (Game|SpawnActorfromClass "/Game/My_BP/BP_SimpleBall.BP_SimpleBall_C" (Math|Transform|MakeTransform (Transformation|GetWorldLocation (Variables|Default|GetCapsule)) "0, 0, 0" "1,1,1") "AlwaysSpawn" 0 0))
  (Variables|Default|SetNewBall _returnvalue))